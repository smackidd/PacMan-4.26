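; GhostBaseBP is the base ghost actor that kills Pac-Man on contact in a Pac-Man style game.
; When its Cylinder overlaps Pac-Man and Pac-Man's Sphere also overlaps the ghost, PacManDead removes a life from ThirdPersonGameMode.
; With no lives left it prints Game Over, pauses and opens the MainMenu level; otherwise it teleports the player and every ghost to hardcoded reset positions.
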(event `self.ReceiveActorBeginOverlap`
  (params (OtherActor :type "Actor Object Reference")))

(event `self.Cylinder.OnComponentBeginOverlap`
  (params (OverlappedComponent :type "PrimitiveComponent Object Reference") (OtherActor :type "Actor Object Reference") (OtherComp :type "PrimitiveComponent Object Reference") (OtherBodyIndex :type Integer) (bFromSweep :type Boolean) (SweepResult :type "HitResult Structure (by ref)"))
  (bind _aspac_man (cast `/Game/Blueprints/PacMan` OtherActor))
  (if (`PrimitiveComponent.IsOverlappingActor` (`/Game/Blueprints/PacMan.Sphere` _aspac_man) self)
    (`self.PacManDead`)))

(fn `PacManDead`
  (bind _asthird_person_game_mode (cast `/Game/ThirdPersonBP/Blueprints/ThirdPersonGameMode` (`GameplayStatics.GetGameMode`)))
  (bind _output_get (set `self.ThirdPersonGameMode` _asthird_person_game_mode))
  (bind _output_get_2 (set `/Game/ThirdPersonBP/Blueprints/ThirdPersonGameMode.Lives` (- (`/Game/ThirdPersonBP/Blueprints/ThirdPersonGameMode.Lives` _output_get) 1) _output_get))
  (if (<= _output_get_2 0)
    (`KismetSystemLibrary.PrintString` "Game Over" true true (struct :`R` 1.0 :`A` 1.0) 20.0)
    (`GameplayStatics.SetGamePaused` true)
    (`GameplayStatics.OpenLevel` "MainMenu")
    (else
      (`self.K2_TeleportTo` :`self` (`GameplayStatics.GetPlayerCharacter` 0) :`DestLocation` (-670.0 -356.44342 202.000671))
      (bind _outactors (`GameplayStatics.GetAllActorsOfClass` "GhostBaseBP_C"))
      (for _array_element _outactors
        (`self.K2_TeleportTo` :`self` _array_element :`DestLocation` (-670.0 234.127991 218.271561))))))

(fn `UserConstructionScript`)