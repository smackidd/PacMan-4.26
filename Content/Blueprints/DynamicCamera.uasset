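; DynamicCamera is a camera actor that becomes player 0's view target on BeginPlay or reset and follows the player character.
; Each Tick moves the spring arm to a per-axis blend of player position and offset-adjusted actor position, weighted by the TrackPlayer vector.
; VInterpTo receives that target with no interp speed set.
; The camera's rotation snaps to look directly at the character using FindLookAtRotation.
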(event `self.ReceiveBeginPlay`
  (`PlayerController.SetViewTargetWithBlend` (`GameplayStatics.GetPlayerController` 0) self 0.0 "VTBlend_Linear" 0.0 false :!label _label)
  (`/Engine/EditorBlueprintResources/StandardMacros.DoOnce` false
    (:`Completed`
      (bind _output_get (set `self.offset` (0.0 200.0 -100.0)))
      (`KismetSystemLibrary.PrintString` (`KismetStringLibrary.Conv_VectorToString` _output_get)))))

(event `self.K2_OnReset`
  (goto _label))

(event `self.ReceiveTick`
  (params (DeltaSeconds :type "Float (single-precision)"))
  (bind _vector (`self.TrackPlayerMovement` DeltaSeconds))
  (`SceneComponent.K2_SetWorldLocation` (`self.SpringArm`) _vector false false)
  (bind _rotation (`self.Track Player Rotation` DeltaSeconds))
  (`SceneComponent.K2_SetWorldRotation` (`self.Camera`) _rotation false false))

(fn `Track Player Rotation`
  (params (Delta :type "Float (double-precision)"))
  (returns (rotation :type "Rotator Structure"))
  (return (`KismetMathLibrary.FindLookAtRotation` (`SceneComponent.K2_GetComponentLocation` (`self.Camera`)) (`self.K2_GetActorLocation` (`GameplayStatics.GetPlayerCharacter` 0)))))

(fn `TrackPlayerMovement`
  (params (DeltaTime :type "Float (double-precision)"))
  (returns (Vector :type "Vector Structure"))
  (bind _trackplayer (`self.TrackPlayer`))
  (bind _returnvalue (- (`self.K2_GetActorLocation`) (`self.offset`)))
  (return (`KismetMathLibrary.VInterpTo` _returnvalue (+ (* (`self.K2_GetActorLocation` (`GameplayStatics.GetPlayerCharacter` 0)) _trackplayer) (* _returnvalue (- (1.0 1.0 1.0) _trackplayer))) DeltaTime)))

(fn `UserConstructionScript`)