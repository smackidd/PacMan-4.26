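; Pac-Man pellet actor that the player collects for points.
; On overlap with PacMan, it adds to the ThirdPersonGameMode score, then hides itself and disables its Sphere collision rather than being destroyed.
; It decrements the game mode's pellet count and calls StartNewLevel when none remain.
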(event `self.ReceiveActorBeginOverlap`
  (params (OtherActor :type "Actor Object Reference"))
  (bind _thirdpersongamemode (`self.ThirdPersonGameMode`))
  ;[1 1 1] detect collision
  (cast `/Game/Blueprints/PacMan` OtherActor)
  (bind _asthird_person_game_mode (cast `/Game/ThirdPersonBP/Blueprints/ThirdPersonGameMode` (`GameplayStatics.GetGameMode`)))
  (bind _output_get (set `self.ThirdPersonGameMode` _asthird_person_game_mode))
  ;[1 1 1] Set Score when eaten
  (set `/Game/ThirdPersonBP/Blueprints/ThirdPersonGameMode.Score` (+ (`/Game/ThirdPersonBP/Blueprints/ThirdPersonGameMode.Score` (`self.ThirdPersonGameMode`)) 10) _output_get)
  ;[1 1 1] Hide Pellets when eaten
  (`self.SetActorHiddenInGame` true)
  (`PrimitiveComponent.SetCollisionEnabled` (`self.Sphere`) "NoCollision")
  ;[1 1 1] Reduce # of pellets left
  (set `/Game/ThirdPersonBP/Blueprints/ThirdPersonGameMode.NumPellets` (- (`/Game/ThirdPersonBP/Blueprints/ThirdPersonGameMode.NumPellets` _thirdpersongamemode) 1) _thirdpersongamemode)
  ;[1 1 1] If all pellets eaten, start new level
  (if (<= (`/Game/ThirdPersonBP/Blueprints/ThirdPersonGameMode.NumPellets` (`self.ThirdPersonGameMode`)) 0)
    (`/Game/ThirdPersonBP/Blueprints/ThirdPersonGameMode.StartNewLevel` (`self.ThirdPersonGameMode`))))

(fn `UserConstructionScript`)